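; BP_Seerr is a seer actor that shows one text component while a Character overlaps its sphere and hides it on exit.
; BeginPlay hides an array of text components, and CurrentIndex, which is never changed here, selects the one to toggle.
; While StartShake is set, Tick calls MakeActorShake to oscillate the Seerr component along X and Y around its starting location using a time-based sine.
; The rotation branch is empty.
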(event `self.ReceiveBeginPlay`
  (bind _first (`self.First`))
  (set `self.SeerOriLoc` (`SceneComponent.K2_GetComponentLocation` (`self.Seerr`)))
  (bind _output_get (set `self.Text_Arr` (`|MakeArray` _first _first (`self.Second`) (`self.Thrird`) (`self.Fourth`))))
  (for _array_element _output_get
    (`SceneComponent.SetVisibility` _array_element false false)))

(event `self.ReceiveTick`
  (params (DeltaSeconds :type "Float (single-precision)"))
  (if (`self.startShake`)
    (`self.MakeActorShake` (`self.Seerr`) (`self.SeerOriLoc`) 600.0 1.0 true)))

(event `self.Sphere.OnComponentBeginOverlap`
  (params (OverlappedComponent :type "PrimitiveComponent Object Reference") (OtherActor :type "Actor Object Reference") (OtherComp :type "PrimitiveComponent Object Reference") (OtherBodyIndex :type Integer) (bFromSweep :type Boolean) (SweepResult :type "HitResult Structure (by ref)"))
  (cast `Character` OtherActor)
  (`SceneComponent.SetVisibility` (`|GetArrayItem` (`self.Text_Arr`) (`self.CurrentIndex`)) true false))

(event `self.Sphere.OnComponentEndOverlap`
  (params (OverlappedComponent :type "PrimitiveComponent Object Reference") (OtherActor :type "Actor Object Reference") (OtherComp :type "PrimitiveComponent Object Reference") (OtherBodyIndex :type Integer))
  (cast `Character` OtherActor)
  (`SceneComponent.SetVisibility` (`|GetArrayItem` (`self.Text_Arr`) (`self.CurrentIndex`)) false false))

(fn `MakeActorShake`
  (params (Target :type "StaticMeshComponent Object Reference") (OriginLoc :type "Vector Structure") (Frequency :type "Float (double-precision)" :default 1.0) (Amplitude :type "Float (double-precision)" :default 1.0) (AffectLoc :type Boolean) (AffectRot :type Boolean))
  (locals (loc :type "Vector Structure" :default (0.0 0.0 0.0)) (rot :type "Rotator Structure" :default (struct)) (SineValue :type "Float (double-precision)"))
  (bind _sinevalue (`local.SineValue`))
  (`|ExecutionSequence`
    (:`then_0`
      (set `local.loc` OriginLoc)
      (set `local.SineValue` (* (`KismetMathLibrary.DegSin` (* (`KismetSystemLibrary.GetGameTimeInSeconds`) (`local.Frequency`))) (`local.Amplitude`))))
    (:`then_1`
      (if AffectLoc
        (`SceneComponent.K2_SetWorldLocation` (`local.Target`) (+ (`local.loc`) (`KismetMathLibrary.MakeVector` _sinevalue _sinevalue)) false false)))
    (:`then_2`
      (if AffectRot
        _))))

(fn `UserConstructionScript`)